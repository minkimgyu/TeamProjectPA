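; Game mode for the zombie map that creates the main HUD widget, runs endless zombie spawning and handles retry and quit.
; A looping timer spawns a girl or police zombie at a random preset transform.
; Spawns and deaths update a live zombie count and refresh its display.
; SpawnAmmo uses a percentage-chance helper to occasionally drop an ammo pickup at a given position.
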(event Custom|QuitGame
  (Game|QuitGame 0 "Quit" false))

(event Custom|SpawnZombies
  ;[1 1 1] Spawn Zombies
  (Utilities|Time|SetTimerbyEvent (delegate Custom|Spawn) 5.0 true))

(event Custom|Retry
  (bind _returnvalue (Game|GetPlayerController 0))
  (Game|OpenLevel(byName) "ZombieMap")
  (Variables|/Script/Engine.PlayerController|SetbShowMouseCursor _returnvalue false)
  (Input|SetInputModeGameOnly _returnvalue false))

(event Custom|ZombieDie
  (Math|Integer|DecrementInt (Variables|Default|GetZombieLeft)
    (:%20%20
      (Default|CallShowZombieCount))))

(event Custom|Spawn
  (bind _spawntransform (Variables|Default|GetSpawnTransform))
  (bind _spawntransform_2 (Variables|Default|GetSpawnTransform))
  (bind _returnvalue (Utilities|Array|Length _spawntransform))
  (bind _returnvalue_2 (Math|Random|RandomInteger _returnvalue))
  (bind _output (Utilities|Array|Get(acopy) _spawntransform_2 _returnvalue_2))
  ;[1 1 1] Spawn Zombies
  (if (== (Math|Random|RandomInteger 2) 1)
    (Game|SpawnActorfromClass "/Game/_Main/Zombies/BaseZombie/BP_GirlZombie.BP_GirlZombie_C" _output "Undefined" 0 0)
    (else
      (Game|SpawnActorfromClass "/Game/_Main/Zombies/BaseZombie/BP_PoliceZombie.BP_PoliceZombie_C" _output "Undefined" 0 0)))
  (Math|Integer|IncrementInt (Variables|Default|GetZombieLeft)
    (:%20%20
      (Default|CallShowZombieCount))))

(event Custom|SpawnAmmo
  (params (position :type Vector))
  ;[1 1 1] Spawn Ammo Crate
  (bind _can (CallFunction|Random 25))
  (if _can
    (Game|SpawnActorfromClass "/Game/_Main/Blueprints/BP_AmmoPickup.BP_AmmoPickup_C" (Math|Transform|MakeTransform position "0, 0, 0" "1.000000,1.000000,1.000000") "Undefined" 0 0)))

(event Custom|Init
  ;[1 1 1] Start Game
  (Utilities|FlowControl|Sequence
    (:then_0
      (bind _returnvalue (UserInterface|CreateWidget "/Game/_Main/Widgets/MainWidget_W.MainWidget_W_C" (Game|GetPlayerController 0)))
      (bind _output_get (Variables|Default|SetMainWidget _returnvalue))
      (UserInterface|Viewport|AddtoViewport _output_get 0))
    (:then_1
      (Default|CallShowZombieCount))
    (:then_2
      (CallFunction|SpawnZombies))))

(event EventTick
  (params (DeltaSeconds :type Float%20%28single-precision%29)))

(event EventBeginPlay
  ;[1 1 1] Widget
  (CallFunction|Init))

(fn ConstructionScript)

(fn Random
  (params (Possibility :type Integer))
  (bind _result (Math|Integer|IncrementInt (Math|Random|RandomInteger 100))
    (:%20%20
      (if (<= _result Possibility)
        (return true)
        (else
          (return false))))))