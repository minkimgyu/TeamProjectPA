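; Player controller that routes the player's combat and movement input to the first-person character.
; On BeginPlay it casts player pawn 0 to BP_FirstPersonCharacter and caches the reference.
; Input actions call that character's functions for shooting, melee, reloading and equipping a pistol or rifle, with Run and Aim passing true on press and false on release.
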(event EventBeginPlay
  (bind _returnvalue (Game|Player|GetPlayerPawn 0))
  (Utilities|IsValid _returnvalue
    (:Is%20Valid
      (bind _asbp_first_person_character (Utilities|Casting|CastToBP_FirstPersonCharacter _returnvalue))
      (Variables|Default|SetFirst%20Person%20Character _asbp_first_person_character))))

(event Input|ActionEvents|InputActionEquipRifle
  (params (Key :type Key%20Structure :default "None"))
  (:Pressed
    (Default|EquipRifle (Variables|Default|GetFirst%20Person%20Character))))

(event Input|ActionEvents|InputActionEquipPistol
  (params (Key :type Key%20Structure :default "None"))
  (:Pressed
    (Default|EquipPistol (Variables|Default|GetFirst%20Person%20Character))))

(event Input|ActionEvents|InputActionReload
  (params (Key :type Key%20Structure :default "None"))
  (:Pressed
    (Default|Reload (Variables|Default|GetFirst%20Person%20Character))))

(event Input|ActionEvents|InputActionShoot
  (params (Key :type Key%20Structure :default "None"))
  (:Pressed
    (Default|Shoot (Variables|Default|GetFirst%20Person%20Character))))

(event Input|ActionEvents|InputActionAim
  (params (Key :type Key%20Structure :default "None"))
  (:Pressed
    (Default|Aim (Variables|Default|GetFirst%20Person%20Character) true))
  (:Released
    (Default|Aim (Variables|Default|GetFirst%20Person%20Character) false)))

(event Input|ActionEvents|InputActionRun
  (params (Key :type Key%20Structure :default "None"))
  (bind _first_person_character (Variables|Default|GetFirst%20Person%20Character))
  (:Pressed
    (Default|Run _first_person_character true))
  (:Released
    (Default|Run _first_person_character false)))

(event Input|ActionEvents|InputActionMeleeAttack
  (params (Key :type Key%20Structure :default "None"))
  (:Pressed
    (Default|MeleeAttack (Variables|Default|GetFirst%20Person%20Character))))

(fn ConstructionScript)