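; Base gun component that handles hitscan firing, ammo, reloading and damage, with stats and montages loaded per gun type from DT_GunDataTable.
; Fire spends a round, line traces from the first-person camera, then blocks further shots until ShootInterval elapses.
; The hit's physical surface selects head or body point damage with blood effects; other surfaces get asphalt particles unless the actor is tagged Zombie, which takes body damage.
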(event Custom|ResetCanShoot
  (Utilities|FlowControl|Delay (Variables|Default|GetShootInterval))
  (Variables|Default|SetCanShoot true))

(fn UseAmmo
  (if (> (Variables|Default|GetCurrentAmmo) 0)
    (Math|Integer|DecrementInt (Variables|Default|GetCurrentAmmo)
      (:%20%20
        (if true
          (return true)
          (else
            (return true)))))
    (else
      (Audio|PlaySound2D 0 1.0 1.0 0.0 0 0)
      (return false))))

(fn LineTracetoObject
  (params (FirstPersonCamera :type Camera%20Component%20Object%20Reference))
  (LocalVariables|SetLocalCameraLocation (Transformation|GetWorldLocation FirstPersonCamera))
  (LocalVariables|SetLocalCameraRotation (Transformation|GetWorldRotation FirstPersonCamera))
  (bind (_outhit _returnvalue) (Collision|LineTraceByChannel (LocalVariables|GetLocalCameraLocation) (+ (LocalVariables|GetLocalCameraLocation) (* (Math|Vector|GetForwardVector (LocalVariables|GetLocalCameraRotation)) (Variables|Default|GetBulletDistance))) "TraceTypeQuery2" true (Utilities|Array|MakeArray 0) "ForDuration"))
  (if _returnvalue
    (Development|PrintString (Utilities|GetDisplayName (.HitActor (Collision|BreakHitResult _outhit))))
    (return _outhit (.Location (Collision|BreakHitResult _outhit)) (.PhysMat (Collision|BreakHitResult _outhit)) (.HitActor (Collision|BreakHitResult _outhit)) (LocalVariables|GetLocalCameraLocation))))

(fn SurfaceDamage
  (params (DamagedActor :type Actor%20Object%20Reference) (HitInfo :type Hit%20Result%20Structure) (Location :type Vector) (Selection :type Physical%20Material%20Object%20Reference) (CameraLocation :type Vector) (DamageCauser :type Actor%20Object%20Reference))
  (bind _surfacetype (Variables|/Script/PhysicsCore.PhysicalMaterial|GetSurfaceType Selection))
  (Utilities|FlowControl|Sequence
    (:then_0
      (LocalVariables|SetLocalDamagedActor DamagedActor))
    (:then_1
      (LocalVariables|SetLocalHitInfo HitInfo))
    (:then_2
      (LocalVariables|SetLocalLocation Location))
    (:then_3
      (LocalVariables|SetLocalCameraLocation CameraLocation))
    (:then_4
      (LocalVariables|SetLocalDamageCauser DamageCauser))
    (:then_5
      (Development|PrintString (Utilities|String|EnumtoString _surfacetype))
      (switch Utilities|FlowControl|Switch|SwitchonEPhysicalSurface _surfacetype
        (:SurfaceType_Default
          (if (not (Actor|ActorHasTag (LocalVariables|GetLocalDamagedActor) "Zombie"))
            (Effects|SpawnEmitteratLocation "/Game/Realistic_Starter_VFX_Pack_Vol2/Particles/Hit/P_Asphalt.P_Asphalt" (LocalVariables|GetLocalLocation))
            (else
              (Utilities|ApplyDamage (LocalVariables|GetLocalDamagedActor) (LocalVariables|GetLocalHitInfo) (Variables|Default|GetBodyDamage) (LocalVariables|GetLocalCameraLocation) (LocalVariables|GetLocalDamageCauser))
              (Effects|SpawnEmitteratLocation "/Game/Realistic_Starter_VFX_Pack_Vol2/Particles/Blood/P_Blood_Splat_Cone.P_Blood_Splat_Cone" (LocalVariables|GetLocalLocation) :!label _label))))
        (:SurfaceType1
          (Utilities|ApplyDamage (LocalVariables|GetLocalDamagedActor) (LocalVariables|GetLocalHitInfo) (Variables|Default|GetHeadDamage) (LocalVariables|GetLocalCameraLocation) (LocalVariables|GetLocalDamageCauser))
          (goto _label))
        (:SurfaceType2
          (Utilities|ApplyDamage (LocalVariables|GetLocalDamagedActor) (LocalVariables|GetLocalHitInfo) (Variables|Default|GetBodyDamage) (LocalVariables|GetLocalCameraLocation) (LocalVariables|GetLocalDamageCauser))
          (goto _label))))))

(fn Reload
  (LocalVariables|SetLocalTempAmmo (Variables|Default|GetCurrentAmmo))
  (Variables|Default|SetCurrentAmmo (Math|Integer|SelectInt (Variables|Default|GetMaxClipSize) (+ (Variables|Default|GetCurrentAmmo) (Variables|Default|GetTotalAmmo)) (>= (+ (Variables|Default|GetCurrentAmmo) (Variables|Default|GetTotalAmmo)) (Variables|Default|GetMaxClipSize))))
  (Variables|Default|SetTotalAmmo (Math|Integer|SelectInt (Math|Integer|Clamp(Integer) (- (Variables|Default|GetTotalAmmo) (- (Variables|Default|GetMaxClipSize) (LocalVariables|GetLocalTempAmmo))) 0 (Variables|Default|GetTotalAmmo)) 0 (>= (+ (Variables|Default|GetCurrentAmmo) (Variables|Default|GetTotalAmmo)) (Variables|Default|GetMaxClipSize)))))

(fn Fire
  (params (FirstPersonCamera :type Camera%20Component%20Object%20Reference) (DamageCauser :type Actor%20Object%20Reference))
  (if (Variables|Default|GetCanShoot)
    (bind _canshoot (CallFunction|UseAmmo))
    (Utilities|FlowControl|Sequence
      (:then_1
        (LocalVariables|SetLocalFirstPersonCamera FirstPersonCamera))
      (:then_2
        (LocalVariables|SetLocalDamageCausor DamageCauser))
      (:then_3
        (if _canshoot
          (Variables|Default|SetCanShoot false)
          (bind (_outhit _location _surfacetype _hitactor _cameralocation) (CallFunction|LineTracetoObject (LocalVariables|GetLocalFirstPersonCamera)))
          (CallFunction|SurfaceDamage _hitactor _outhit _location _surfacetype _cameralocation (LocalVariables|GetLocalDamageCausor))
          (CallFunction|ResetCanShoot)
          (return true)
          (else
            (return false)))))
    (else
      (return false))))

(fn CanReload
  (return (not (or (== (Variables|Default|GetCurrentAmmo) (Variables|Default|GetMaxClipSize)) (<= (Variables|Default|GetTotalAmmo) 0)))))

(fn InitDatafromTable
  (params (Type :type GunType%20Enum :default "NewEnumerator0"))
  (bind _returnvalue (Utilities|GetDataTableRow "/Game/_Main/Blueprints/Gun/DT_GunDataTable.DT_GunDataTable" (Utilities|String|StringToName (Utilities|String|EnumtoString Type)))
    (:then
      (Utilities|FlowControl|Sequence
        (:then_0
          (bind _output_get (Variables|Default|SetMaxClipSize (.maxclipsize _returnvalue)))
          (Variables|Default|SetCurrentAmmo _output_get))
        (:then_1
          (Variables|Default|SetTotalAmmo (.totalammo _returnvalue)))
        (:then_2
          (Variables|Default|SetBodyDamage (.bodydamage _returnvalue)))
        (:then_3
          (Variables|Default|SetHeadDamage (.headdamage _returnvalue)))
        (:then_4
          (Variables|Default|SetBulletDistance (.bulletdistance _returnvalue)))
        (:then_5
          (Variables|Default|SetAimFireMontage (.aimfiremontage _returnvalue)))
        (:then_6
          (Variables|Default|SetIdleFireMontage (.idlefiremontage _returnvalue)))
        (:then_7
          (Variables|Default|SetReloadMontage (.reloadmontage _returnvalue)))
        (:then_8
          (Variables|Default|SetSwingDamage (.swingdamage _returnvalue)))
        (:then_9
          (Variables|Default|SetShootInterval (.shootinterval _returnvalue)))
        (:then_10
          (Variables|Default|SetSwingInterval (.swinginterval _returnvalue)))))))

(fn AddAmmo
  (Variables|Default|SetTotalAmmo (+ (Variables|Default|GetTotalAmmo) (Variables|Default|GetMaxClipSize))))