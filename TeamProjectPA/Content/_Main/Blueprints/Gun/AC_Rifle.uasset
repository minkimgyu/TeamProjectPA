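; Actor component that gives the rifle a melee swing, allowed only when not aiming and for one specific gun type.
; Swing runs a sphere overlap for Pawns at an arrow's location, ignoring the wielder, and damages the first hit before returning true.
; A CanSwing flag gates the attack, and the ResetSwing event restores it after the swing interval, whether or not anything was hit.
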(event Custom|ResetSwing
  (params (SwingInterval :type Float%20%28double-precision%29))
  (Utilities|FlowControl|Delay SwingInterval)
  (Variables|Default|SetCanSwing true))

(fn Swing
  (params (IsAiming :type Boolean) (GunType :type GunType%20Enum :default "NewEnumerator0") (Arrow :type Arrow%20Component%20Object%20Reference) (FirstPerson :type Actor%20Object%20Reference) (SwingDamage :type Float%20%28double-precision%29) (SwingInterval :type Float%20%28double-precision%29))
  (LocalVariables|SetLocalSwingInterval SwingInterval)
  (LocalVariables|SetLocalSwingDamage SwingDamage)
  (if (Variables|Default|GetCanSwing)
    (if (and (not IsAiming) (Utilities|Enum|Equal(Enum) GunType "NewEnumerator1"))
      (Variables|Default|SetCanSwing false)
      (LocalVariables|SetLocalFirstPerson FirstPerson)
      (bind (_outactors _returnvalue) (Collision|SphereOverlapActors (Transformation|GetWorldLocation Arrow) 8e+01 (Utilities|Array|MakeArray "ObjectTypeQuery3") 0 (Utilities|Array|MakeArray (LocalVariables|GetLocalFirstPerson))))
      (if _returnvalue
        (for _array_element _outactors
          (Game|Damage|ApplyDamage _array_element (LocalVariables|GetLocalSwingDamage) (Game|GetInstigatorController (LocalVariables|GetLocalFirstPerson)) (LocalVariables|GetLocalFirstPerson))
          (CallFunction|ResetSwing (LocalVariables|GetLocalSwingInterval))
          (return true))
        (else
          (CallFunction|ResetSwing (LocalVariables|GetLocalSwingInterval))
          (return true)))
      (else
        (return false)))
    (else
      (return false))))