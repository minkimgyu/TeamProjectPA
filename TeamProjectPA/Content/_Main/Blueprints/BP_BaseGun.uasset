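; Base gun Blueprint for shooting zombies with hitscan fire, providing Fire and Reload functions with ammo tracking.
; Fire spends a round unless empty or reloading, then line traces from the first-person camera.
; The hit physical material's surface type selects head or body point damage with blood effects, while other untagged hits spawn asphalt impacts.
; Reload flags the reloading state and refills the clip from reserve ammo.
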(fn ConstructionScript)

(fn UseAmmo
  (if (> (Variables|Default|GetCurrentAmmo) 0)
    (if (not (Variables|Default|GetIsReloading))
      (Math|Integer|DecrementInt (Variables|Default|GetCurrentAmmo)
        (:%20%20
          (if (Variables|Default|GetIsAiming)
            (return true true)
            (else
              (return false true))))))
    (else
      (Audio|PlaySound2D 0 1.0 1.0 0.0 0 0)
      (return false false))))

(fn LineTracetoObject
  (params (FirstPersonCamera :type Camera%20Component%20Object%20Reference))
  (Variables|Default|SetCameraLocation (Transformation|GetWorldLocation FirstPersonCamera))
  (LocalVariables|SetLocalCameraRotation (Transformation|GetWorldRotation FirstPersonCamera))
  (bind (_outhit _returnvalue) (Collision|LineTraceByChannel (Variables|Default|GetCameraLocation) (+ (Variables|Default|GetCameraLocation) (* (Math|Vector|GetForwardVector (LocalVariables|GetLocalCameraRotation)) (Variables|Default|GetBulletDistance))) "TraceTypeQuery2" true (Utilities|Array|MakeArray self) "ForDuration"))
  (if _returnvalue
    (return _outhit (.Location (Collision|BreakHitResult _outhit)) (Variables|/Script/PhysicsCore.PhysicalMaterial|GetSurfaceType (.PhysMat (Collision|BreakHitResult _outhit))) (.HitActor (Collision|BreakHitResult _outhit)) 0)))

(fn SurfaceDamage
  (params (DamagedActor :type Actor%20Object%20Reference) (HitInfo :type Hit%20Result%20Structure) (Location :type Vector) (Selection :type EPhysicalSurface%20Enum :default "SurfaceType_Default"))
  (Utilities|FlowControl|Sequence
    (:then_0
      (LocalVariables|SetLocalDamagedActor DamagedActor))
    (:then_1
      (LocalVariables|SetLocalHitInfo HitInfo))
    (:then_2
      (LocalVariables|SetLocalLocation Location))
    (:then_3
      (switch Utilities|FlowControl|Switch|SwitchonEPhysicalSurface Selection
        (:SurfaceType_Default
          (if (not (Actor|ActorHasTag (LocalVariables|GetLocalDamagedActor) "Zombie"))
            (Effects|SpawnEmitteratLocation "/Game/Realistic_Starter_VFX_Pack_Vol2/Particles/Hit/P_Asphalt.P_Asphalt" (LocalVariables|GetLocalLocation))
            (else
              (Utilities|ApplyDamage (LocalVariables|GetLocalDamagedActor) (LocalVariables|GetLocalHitInfo) 0.0)
              (Effects|SpawnEmitteratLocation "/Game/Realistic_Starter_VFX_Pack_Vol2/Particles/Blood/P_Blood_Splat_Cone.P_Blood_Splat_Cone" (LocalVariables|GetLocalLocation) :!label _label))))
        (:SurfaceType1
          (Utilities|ApplyDamage (LocalVariables|GetLocalDamagedActor) (LocalVariables|GetLocalHitInfo) (Variables|Default|GetHeadDamage))
          (goto _label))
        (:SurfaceType2
          (Utilities|ApplyDamage (LocalVariables|GetLocalDamagedActor) (LocalVariables|GetLocalHitInfo) (Variables|Default|GetBodyDamage))
          (goto _label))))))

(fn Reload
  (if (or (== (Variables|Default|GetCurrentAmmo) (Variables|Default|GetMaxClipSize)) (<= (Variables|Default|GetTotalAmmo) 0))
    (return false)
    (else
      (Variables|Default|SetIsReloading true)
      (LocalVariables|SetLocalTempAmmo (Variables|Default|GetCurrentAmmo))
      (Variables|Default|SetCurrentAmmo (Math|Integer|SelectInt (Variables|Default|GetMaxClipSize) (+ (Variables|Default|GetCurrentAmmo) (Variables|Default|GetTotalAmmo)) (>= (+ (Variables|Default|GetCurrentAmmo) (Variables|Default|GetTotalAmmo)) (Variables|Default|GetMaxClipSize))))
      (Variables|Default|SetTotalAmmo (Math|Integer|SelectInt (Math|Integer|Clamp(Integer) (- (Variables|Default|GetTotalAmmo) (- (Variables|Default|GetMaxClipSize) (LocalVariables|GetLocalTempAmmo))) 0 (Variables|Default|GetTotalAmmo)) 0 (>= (+ (Variables|Default|GetCurrentAmmo) (Variables|Default|GetTotalAmmo)) (Variables|Default|GetMaxClipSize))))
      (return true))))

(fn Fire
  (params (FirstPersonCamera :type Camera%20Component%20Object%20Reference))
  (bind (_nowaiming _canshoot) (CallFunction|UseAmmo))
  (Utilities|FlowControl|Sequence
    (:then_0
      (LocalVariables|SetLocalNowAiming _nowaiming))
    (:then_1
      (LocalVariables|SetLocalFirstPersonCamera FirstPersonCamera))
    (:then_2
      (if _canshoot
        (bind (_outhit _location _surfacetype _hitactor) (CallFunction|LineTracetoObject))
        (CallFunction|SurfaceDamage _hitactor _outhit _location _surfacetype)
        (return true (LocalVariables|GetLocalNowAiming))
        (else
          (return false (LocalVariables|GetLocalNowAiming)))))))